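; BP_Walls_Level1 is a platformer wall prop that snaps itself to a fixed height for its level.
; When UseSnap is on, the construction script keeps the actor's X and Y and overrides Z based on the Level value.
; Level 0 and unhandled values share the base height, while level 1 sits higher, raised further when UseFloorSpacing is set.
; The event graph holds no active logic.
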(event EventBeginPlay)

(event Collision|EventActorBeginOverlap
  (params (OtherActor :type Actor%20Object%20Reference)))

(event EventTick
  (params (DeltaSeconds :type Float%20%28single-precision%29)))

(fn ConstructionScript
  (bind _returnvalue (Transformation|GetActorLocation))
  (bind _returnvalue_2 (Transformation|GetActorLocation))
  (bind _returnvalue_3 (Transformation|GetActorLocation))
  (if (Variables|Default|GetbUseSnap)
    (switch int (Variables|Default|GetLevel)
      (:Default
        (Transformation|SetActorLocation (Math|Vector|MakeVector (.x _returnvalue_2) (.y _returnvalue_2) 5e+01) false false :!label _label))
      (:0
        (goto _label))
      (:1
        (if (Variables|Default|GetbUseFloorSpacing)
          (Transformation|SetActorLocation (Math|Vector|MakeVector (.x _returnvalue_3) (.y _returnvalue_3) 3e+02) false false)
          (else
            (Transformation|SetActorLocation (Math|Vector|MakeVector (.x _returnvalue) (.y _returnvalue) 2.5e+02) false false)))))))