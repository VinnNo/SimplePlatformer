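; Player character Blueprint that connects interaction, item collection and dialogue to the game's UI and animation.
; BeginPlay creates the mobile HUD, touch buttons and optional debug widget, which displays physics state, substate and launch combo through bound dispatchers.
; Events update key count and touch prompts, play the collect animation, and show or remove locked-door dialogue.
; Hardcoded keys trigger interact, cancel or quit.
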(event Custom|BindEvents
  ;[1 1 1] Debug Stuff
  (EventDispatchers|AssignOnPhysicsStateChanged (delegate Custom|OnPhysicsStateChanged_Event_0))
  (EventDispatchers|AssignOnSubstateChanged (delegate Custom|OnSubstateChanged_Event_0))
  (EventDispatchers|AssignOnLaunchedCharacter (delegate Custom|OnLaunchedCharacter_Event_0)))

(event Custom|OnPhysicsStateChanged_Event_0
  (params (State :type EPhysicsStates%20Enum :default "Idle") (StateString :type String))
  ;[1 1 1] Debug Stuff
  (Default|SetState (Variables|Default|GetDebugUI) StateString))

(event Custom|OnSubstateChanged_Event_0
  (params (StateString :type String))
  ;[1 1 1] Debug Stuff
  (Default|SetSubstate (Variables|Default|GetDebugUI) StateString))

(event Custom|OnLaunchedCharacter_Event_0
  (params (Combo :type Integer) (Multiplier :type Float%20%28single-precision%29))
  (bind _debugui (Variables|Default|GetDebugUI))
  ;[1 1 1] Debug Stuff
  (Default|SetCombo _debugui Combo)
  (Default|SetComboMultiplier _debugui Multiplier))

(event Custom|SpawnWidgets
  (Utilities|FlowControl|Sequence
    (:then_0
      (if (Variables|Default|GetbIsDebug)
        (bind _returnvalue (UserInterface|CreateWidget "/Game/BP/Blueprints/WBP_DebugWidget.WBP_DebugWidget_C"))
        (Variables|Default|SetDebugUI _returnvalue)))
    (:then_1
      (bind _returnvalue_2 (UserInterface|CreateWidget "/Game/BP/Blueprints/WBP_Temp_Touch.WBP_Temp_Touch_C"))
      (Variables|Default|SetTouchButtons _returnvalue_2))
    (:then_2
      (bind _returnvalue_3 (UserInterface|CreateWidget "/Game/BP/Blueprints/WBP_Game_HudMobile.WBP_Game_HudMobile_C"))
      (Variables|Default|SetGameHud _returnvalue_3))
    (:then_3
      (CallFunction|AddWidgetstoViewPort))))

(event Custom|CancelInteraction
  (Class|CharacterBase|InputCancelInteraction))

(event Custom|AddWidgetsToViewPort
  (Utilities|FlowControl|Sequence
    (:then_0
      (UserInterface|Viewport|AddtoViewport (Variables|Default|GetGameHud) 0))
    (:then_1
      (UserInterface|Viewport|AddtoViewport (Variables|Default|GetDebugUI) 0))
    (:then_2
      (UserInterface|Viewport|AddtoViewport (Variables|Default|GetTouchButtons) 2))))

(event Custom|Interact
  (Class|CharacterBase|InputInteraction))

(event EventBeginPlay
  (CallFunction|BindEvents)
  (CallFunction|SpawnWidgets))

(event Collision|EventActorBeginOverlap
  (params (OtherActor :type Actor%20Object%20Reference)))

(event EventUpdateSmallKeyCount
  (Class|WinGameHud|UpdateSmallKeyCount (Variables|Default|GetGameHud) (Utilities|Array|Length (Variables|/Script/SimplePlatformer.InventoryComponent|GetSmallKeys (Variables|Default|GetInventory)))))

(event EventOnInteractionChanged
  (Class|WMobileButtons|UpdateInteractionType (Variables|Default|GetTouchButtons) (Variables|Default|GetInteractableType) false))

(event EventSpawnActiveDialogue
  (bind _returnvalue (UserInterface|CreateWidget (Variables|Default|GetActiveDialogue)))
  (bind _output_get (Variables|Default|SetDialogue _returnvalue))
  (bind _aswbp_dialogue_locked_door (Utilities|Casting|CastToWBP_Dialogue_LockedDoor _output_get))
  (Default|SetWidgetDefaults _aswbp_dialogue_locked_door (Utilities|Array|Length (Variables|/Script/SimplePlatformer.InventoryComponent|GetSmallKeys (Variables|Default|GetInventory))))
  (UserInterface|Viewport|AddtoViewport _output_get 0))

(event EventRemoveActiveDialogue
  (bind _aswbp_dialogue_locked_door (Utilities|Casting|CastToWBP_Dialogue_LockedDoor (Variables|Default|GetDialogue)))
  (Default|RemoveSelf _aswbp_dialogue_locked_door))

(event EventOnItemCollectStarted
  (bind _mesh (Variables|Character|GetMesh))
  (Components|Animation|SetAnimationMode _mesh "AnimationSingleNode")
  (Components|Animation|PlayAnimation _mesh "/Game/Platformer/Character/Fox/Anim_Item_Collect.Anim_Item_Collect" false))

(event EventOnItemCollectFinished
  (Components|Animation|SetAnimationMode (Variables|Character|GetMesh) "AnimationBlueprint"))

(event Input|KeyboardEvents|C
  (params (Key :type Key%20Structure :default "None"))
  (:Pressed
    (CallFunction|Interact)))

(event Input|KeyboardEvents|AndroidBack
  (params (Key :type Key%20Structure :default "None"))
  (:Pressed
    (Game|QuitGame 0 "Quit" false)))

(event Input|KeyboardEvents|Escape
  (params (Key :type Key%20Structure :default "None"))
  (:Pressed
    (Game|QuitGame 0 "Quit" false)))

(event Input|KeyboardEvents|X
  (params (Key :type Key%20Structure :default "None"))
  (:Pressed
    (CallFunction|CancelInteraction)
    (Development|PrintString (Utilities|String|ToString(Vector) (Transformation|GetWorldLocation (Variables|Default|GetCameraComp))))))

(fn ConstructionScript)